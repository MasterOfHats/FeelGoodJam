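; Affinity meter actor that shows a table's relationship or heartbreak progress as camera-facing heart sprites.
; Tick shows both hearts for In Relationship or only the first for Heartbroken, and hides them when opacity is zero or the table is inactive.
; Meter functions tint hearts from grey by affinity, with relationship affinity also driving their separation through a mirrored timeline lerp.
; CakeReaction, BeginRelationship and ChangeOpacity are stubs.
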(event Custom|MoveHeartsRelative
  (params (NewRelativeLocation :type Vector))
  (Variables|Default|SetNewLoc NewRelativeLocation)
  (Variables|Default|SetOldLoc (Variables|/Script/Engine.SceneComponent|GetRelativeLocation (Variables|Default|Get%20Individual1_Heart)))
  (Components|Timeline|SetPlayRate (Variables|Default|GetMovingTimeline) (/ 1.0 (Variables|Default|GetMoveTime)))
  (bind _lerp (Timeline|MovingTimeline PlayFromStart)
    (:Update
      (Transformation|SetRelativeLocation (Variables|Default|Get%20Individual1_Heart) (Math|Vector|Lerp(Vector) (Variables|Default|GetOldLoc) (Variables|Default|GetNewLoc) _lerp) false false)
      (Transformation|SetRelativeLocation (Variables|Default|Get%20Individual2_Heart) (* (Math|Vector|Lerp(Vector) (Variables|Default|GetOldLoc) (Variables|Default|GetNewLoc) _lerp) -1.0) false false))))

(event Custom|ChangeOpacity
  (params (Opacity :type Float%20%28single-precision%29)))

(event EventBeginPlay
  (Variables|Default|SetCameraManager (Game|GetPlayerCameraManager 0))
  (bind _output_get (Variables|Default|SetCurrentColor (Variables|Default|GetBaseColor)))
  (CallFunction|SetHeartColors _output_get))

(event EventTick
  (params (DeltaSeconds :type Float%20%28single-precision%29))
  (bind _table (Variables|Default|GetTable))
  (bind _individual1 (Variables|/Game/FGJ/Core/BP_Table.BP_Table_C|GetIndividual1 _table))
  (if (and (!= (Variables|Default|GetCurrentOpacity) 0.0) (Variables|/Game/FGJ/Core/BP_Table.BP_Table_C|GetTableActive (Variables|Default|GetTable)))
    (Utilities|FlowControl|Sequence
      (:then_0
        (CallFunction|FaceCamera))
      (:then_1
        (Utilities|IsValid _individual1
          (:Is%20Valid
            (switch Utilities|FlowControl|Switch|SwitchonEIndividualStatus (Variables|/Game/FGJ/AI/BP_Individual.BP_Individual_C|GetStatus _individual1)
              (:NewEnumerator0
                (Rendering|SetVisibility (Variables|Default|Get%20Individual1_Heart) true false))
              (:NewEnumerator1
                (Rendering|SetVisibility (Variables|Default|Get%20Individual1_Heart) true false)
                (Rendering|SetVisibility (Variables|Default|Get%20Individual2_Heart) false false)))))))
    (else
      (Rendering|SetVisibility (Variables|Default|Get%20Individual1_Heart) false false))))

(fn ConstructionScript)

(fn RelationshipMeter
  (params (Affinity :type Integer))
  (bind _table (Variables|Default|GetTable))
  (bind _maxrelationshipaffinity (Variables|/Game/FGJ/Core/BP_Table.BP_Table_C|GetMaxRelationshipAffinity _table))
  (CallFunction|SetHeartColors (Class|KismetMathLibrary|LinearColorLerpUsingHSV (Variables|Default|GetGreyedColor) (Variables|Default|GetBaseColor) (* Affinity (/ 1.0 (* (Math|Conversions|ToFloat(Integer) (Variables|/Game/FGJ/Core/BP_Table.BP_Table_C|GetMaxRelationshipAffinity (Variables|Default|GetTable))) 0.33)))))
  (CallFunction|MoveHearts (Math|Vector|MakeVector 0.0 (Math|Float|Lerp 0.0 (/ (Variables|Default|GetRelationshipHeartMaxDistance) 2.0) (* (Math|Conversions|ToFloat(Integer) (- Affinity _maxrelationshipaffinity)) (/ 1.0 (Math|Conversions|ToFloat(Integer) _maxrelationshipaffinity)))) 0.0)))

(fn HeartbreakMeter
  (params (Affinity :type Integer))
  (CallFunction|SetHeartColors (Class|KismetMathLibrary|LinearColorLerpUsingHSV (Variables|Default|GetGreyedColor) (Variables|Default|GetBaseColor) (* Affinity (/ 1.0 (Math|Conversions|ToFloat(Integer) (Variables|/Game/FGJ/AI/BP_Individual.BP_Individual_C|GetMaxHeartbreakAffinity (Variables|/Game/FGJ/Core/BP_Table.BP_Table_C|GetIndividual1 (Variables|Default|GetTable)))))))))

(fn CakeReaction
  (params (Affinity :type Integer))
  (if (not (== Affinity -5))
    (if (not (== Affinity -2))
      (if (not (== Affinity 2))
        (if (not (== Affinity 5))
          (if (not (== Affinity 10))
            (Development|PrintString "Affinity out of bounds")))))))

(fn SetHeartColors
  (params (NewColor :type Linear%20Color%20Structure))
  (bind _output_get (Variables|Default|SetCurrentColor (Utilities|Struct|MakeLinearColor (.r NewColor) (.g NewColor) (.b NewColor) (Variables|Default|GetCurrentOpacity))))
  (Sprite|SetSpriteColor (Variables|Default|Get%20Individual1_Heart) _output_get))

(fn SetHeartOpacities
  (params (NewOpacity :type Float%20%28single-precision%29))
  (Variables|Default|SetCurrentOpacity NewOpacity)
  (CallFunction|SetHeartColors (Variables|Default|GetCurrentColor)))

(fn FaceCamera
  (bind _returnvalue (Transformation|GetActorLocation))
  (bind _cameramanager (Variables|Default|GetCameraManager))
  (bind _returnvalue_2 (Camera|GetCameraLocation _cameramanager))
  (bind _returnvalue_3 (Math|Rotator|FindLookatRotation _returnvalue_2 _returnvalue))
  (Transformation|SetActorRotation (Math|Rotator|MakeRotator (.roll _returnvalue_3) (.pitch _returnvalue_3) (.yaw _returnvalue_3))))

(fn MoveHearts
  (params (NewRelativeLocation :type Vector))
  (CallFunction|MoveHeartsRelative NewRelativeLocation))

(fn BeginRelationship)

(fn BeginHeartbreak
  (CallFunction|MoveHearts "0, 0, 0")
  (Development|PrintString "set hearts to 0"))