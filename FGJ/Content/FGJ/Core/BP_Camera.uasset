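; BP_Camera is a camera actor that switches behavior each tick on CameraMode, Overview or Cake.
; Overview follows the player pawn, mapping its Y to camera sideways offset and its X to pitch within set bounds, each smoothed with FInterpTo.
; Cake yaws the whole actor when the mouse enters the left or right screen margins, turning faster toward the edge.
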(event EventBeginPlay)

(event EventTick
  (params (DeltaSeconds :type Float%20%28single-precision%29))
  (bind _returnvalue (Utilities|Time|GetWorldDeltaSeconds))
  (switch Utilities|FlowControl|Switch|SwitchonCameraMode (Variables|Default|GetCameraMode)
    (:NewEnumerator0
      (CallFunction|AdjustOverview))
    (:NewEnumerator1
      (bind _returnvalue_2 (Class|WidgetLayoutLibrary|GetMousePositiononViewport))
      (if (< (.X (Math|Vector2D|BreakVector2D (/ (* _returnvalue_2 (Class|WidgetLayoutLibrary|GetViewportScale)) (Viewport|GetViewportSize)))) 0.3)
        (Transformation|AddActorLocalRotation (Math|Rotator|MakeRotator 0.0 0.0 (* (Math|Float|MapRangeClamped (.X (Math|Vector2D|BreakVector2D (/ (* _returnvalue_2 (Class|WidgetLayoutLibrary|GetViewportScale)) (Viewport|GetViewportSize)))) 0.3 0.0 0.0 -1.2e+02) _returnvalue)) false false)
        (elif (> (.X (Math|Vector2D|BreakVector2D (/ (* _returnvalue_2 (Class|WidgetLayoutLibrary|GetViewportScale)) (Viewport|GetViewportSize)))) 0.7)
          (Transformation|AddActorLocalRotation (Math|Rotator|MakeRotator 0.0 0.0 (* _returnvalue (Math|Float|MapRangeClamped (.X (Math|Vector2D|BreakVector2D (/ (* _returnvalue_2 (Class|WidgetLayoutLibrary|GetViewportScale)) (Viewport|GetViewportSize)))) 0.7 1.0 0.0 1.2e+02))) false false))))))

(fn ConstructionScript)

(fn AdjustOverview
  (bind _returnvalue (Game|Player|GetPlayerPawn 0))
  (bind _anglerange (Variables|Default|GetAngleRange))
  (bind _translationrange (Variables|Default|GetTranslationRange))
  (bind _camera (Variables|Default|GetCamera))
  (bind (_lowerbound _upperbound) (Utilities|Struct|BreakFloatRange _translationrange))
  (bind (_lowerbound_2 _upperbound_2) (Utilities|Struct|BreakFloatRange _anglerange))
  (bind _returnvalue_2 (Transformation|GetActorLocation _returnvalue))
  (Transformation|SetRelativeLocationAndRotation _camera (Math|Vector|MakeVector 0.0 (Math|Interpolation|FInterpTo (.y (Variables|/Script/Engine.SceneComponent|GetRelativeLocation (Variables|Default|GetCamera))) (Math|Float|MapRangeClamped (.y _returnvalue_2) (Variables|Default|GetCameraBoundsLeft) (Variables|Default|GetCameraBoundsRight) (.value _lowerbound) (.value _upperbound)) (Utilities|Time|GetWorldDeltaSeconds) 4.0) 0.0) (Math|Rotator|MakeRotator 0.0 (Math|Interpolation|FInterpTo (.pitch (Variables|/Script/Engine.SceneComponent|GetRelativeRotation _camera)) (Math|Float|MapRangeClamped (.x _returnvalue_2) (Variables|Default|GetCameraBoundsDown) (Variables|Default|GetCameraBoundsUp) (.value _lowerbound_2) (.value _upperbound_2)) (Utilities|Time|GetWorldDeltaSeconds) 1.0) 0.0) false false))