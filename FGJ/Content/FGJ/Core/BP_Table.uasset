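; Cafe table actor that seats individuals and runs either a two-person relationship or a solo heartbreak.
; A delayed self-looping Progress event shifts affinity, while Tick checks thresholds to end relationships in departure or breakup, or heartbreak in Waiting status.
; Given cake is scored against the table's random emoji by BP_MainGameMode, then a timeline shrinks it while adding affinity in steps.
; Breakups leave both partners heartbroken, moving the second to another table.
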(event Custom|Progress
  (bind _affinityprogresstimerange (Variables|Default|GetAffinityProgressTimeRange))
  ;[1 1 1] Loops During Relationship & Heartbroken states
  (switch Utilities|FlowControl|Switch|SwitchonEIndividualStatus (Variables|/Game/FGJ/AI/BP_Individual.BP_Individual_C|GetStatus (Variables|Default|GetIndividual1))
    (:NewEnumerator0
      (CallFunction|ProgressRelationship))
    (:NewEnumerator1
      (CallFunction|ProgressHeartbreak)))
  (Utilities|FlowControl|Delay (Math|Random|RandomFloatinRange (.x _affinityprogresstimerange) (.y _affinityprogresstimerange)))
  (if (Variables|Default|GetcanProgress)
    (CallFunction|Progress)))

(event Custom|EatCake
  (bind _cakeeatingtimerange (Variables|Default|GetCakeEatingTimeRange))
  ;[1 1 1] Event EatCake - Calculates affinity then lerps cake to consumption, staggering adding affinity
  (bind _affinity (Default|CalculateAffinity (Variables|Default|GetGameMode) (Variables|Default|GetCurrentEmoji) (Variables|Default|GetCurrentCake)))
  (switch Utilities|FlowControl|Switch|SwitchonEIndividualStatus (Variables|/Game/FGJ/AI/BP_Individual.BP_Individual_C|GetStatus (Variables|Default|GetIndividual1))
    (:NewEnumerator0
      (Variables|Default|SetCakeAffinityPositive (> _affinity 0) :!label _label)
      (bind _output_get (Variables|Default|SetCakeEatingAffinityStep (/ 1.0 (Math|Conversions|ToFloat(Integer) _affinity)))))
    (:NewEnumerator1
      ;;[1 1 1] If cake is negative with a heartbroken individual then set it to affinity gain to 1
      (if (< _affinity 0)
        (Variables|Default|SetCakeAffinityPositive true)
        (Variables|Default|SetCakeEatingAffinityStep (/ 1.0 (Math|Conversions|ToFloat(Integer) 1)))
        (else
          (goto _label)))))
  (Variables|Default|SetCakeEatingAffinityStepCounter _output_get)
  (Components|Timeline|SetPlayRate (Variables|Default|GetEatingCakeTimeline) (Math|Random|RandomFloatinRange (.x _cakeeatingtimerange) (.y _cakeeatingtimerange)))
  (bind _cakeshrinkalpha (Timeline|EatingCakeTimeline Play)
    (:Update
      (Transformation|SetActorScale3D (Variables|Default|GetCurrentCake) (Math|Vector|MakeVector (Math|Float|Lerp 1.0 0.1 _cakeshrinkalpha) (Math|Float|Lerp 1.0 0.1 _cakeshrinkalpha) (Math|Float|Lerp 1.0 0.1 _cakeshrinkalpha)))
      (if (>= (Variables|Default|GetCakeEatingAffinityStepCounter) _cakeshrinkalpha)
        (Variables|Default|SetCakeEatingAffinityStepCounter (+ (Variables|Default|GetCakeEatingAffinityStepCounter) (Variables|Default|GetCakeEatingAffinityStep)))
        (if (Variables|Default|GetCakeAffinityPositive)
          (CallFunction|AddAffinity 1)
          (else
            (CallFunction|AddAffinity -1)))
        (Development|PrintString "Adding Affinity")))
    (:Finished
      (Default|PoofCake (Variables|Default|GetCurrentCake))
      (CallFunction|CakeEaten))))

(event EventBeginPlay
  (bind _asbp_main_game_mode (Utilities|Casting|CastToBP_MainGameMode (Game|GetGameMode)))
  (Variables|Default|SetGameMode _asbp_main_game_mode))

(event EventTick
  (params (DeltaSeconds :type Float%20%28single-precision%29))
  (bind _individual1 (Variables|Default|GetIndividual1))
  (bind _tablewaitingrange (Variables|Default|GetTableWaitingRange))
  (bind _tablewaitingrange_2 (Variables|Default|GetTableWaitingRange))
  (bind _tablewaitingrange_3 (Variables|Default|GetTableWaitingRange))
  (if (Variables|Default|GetTableActive)
    (switch Utilities|FlowControl|Switch|SwitchonEIndividualStatus (Variables|/Game/FGJ/AI/BP_Individual.BP_Individual_C|GetStatus (Variables|Default|GetIndividual1))
      (:NewEnumerator0
        ;[1 1 1] Check relationship, progress relationship, if cake then slowly add that to affinity as well
        (if (Variables|Default|GetWaitingForPartner)
          (Development|PrintString "WAITING")
          (elif (>= (Variables|Default|GetRelationshipAffinity) (Variables|Default|GetMaxRelationshipAffinity))
            ;;[1 1 1] Relationship Succeeded - Wait a while before leaving
            (CallFunction|TableWaitingFinish)
            (Utilities|FlowControl|Delay (Math|Random|RandomFloatinRange (.x _tablewaitingrange_2) (.y _tablewaitingrange_2)))
            (CallFunction|FinishRelationship true)
            (elif (<= (Variables|Default|GetRelationshipAffinity) 0)
              ;;[1 1 1] Relationship Failed - Wait a while before breaking up
              (Development|PrintString "FAILED")
              (CallFunction|TableWaitingFinish)
              (Utilities|FlowControl|Delay (Math|Random|RandomFloatinRange (.x _tablewaitingrange_3) (.y _tablewaitingrange_3)))
              (CallFunction|FinishRelationship false)))))
      (:NewEnumerator1
        ;[1 1 1] Progress Heartbreak, if cake then slowly add that to affinity as well
        (if (>= (Variables|/Game/FGJ/AI/BP_Individual.BP_Individual_C|GetHeartbreakAffinity _individual1) (Variables|/Game/FGJ/AI/BP_Individual.BP_Individual_C|GetMaxHeartbreakAffinity _individual1))
          ;;[1 1 1] Heart heals, after a time switch to waiting status
          (CallFunction|TableWaitingFinish)
          (Utilities|FlowControl|Delay (Math|Random|RandomFloatinRange (.x _tablewaitingrange) (.y _tablewaitingrange)))
          (CallFunction|FinishHeartbreak))))))

(fn ConstructionScript)

(fn IndividualMovingtoTable
  (params (Individual :type BP%20Individual%20Object%20Reference))
  (Variables|Default|SetTableTaken true)
  (switch Utilities|FlowControl|Switch|SwitchonEIndividualStatus (Variables|/Game/FGJ/AI/BP_Individual.BP_Individual_C|GetStatus Individual)
    (:NewEnumerator0
      (Variables|BP_Table_C|SetCoupleIsBeside (Variables|Default|GetPairedTable) true))))

(fn IndividualSatDown
  (params (Individual :type BP%20Individual%20Object%20Reference))
  (if (Variables|Default|GetWaitingForPartner)
    (Development|PrintString "Second  Indiviidual sat down" true true "(R=0.000000,G=0.660000,B=1.000000,A=1.000000)" 5.0)
    (Variables|Default|SetIndividual2 Individual)
    (Variables|Default|SetWaitingForPartner false)
    (CallFunction|SetupTable)
    (else
      (Development|PrintString "First Indiviidual sat down" true true "(R=0.000000,G=0.660000,B=1.000000,A=1.000000)" 5.0)
      (bind _output_get (Variables|Default|SetIndividual1 Individual))
      (switch Utilities|FlowControl|Switch|SwitchonEIndividualStatus (Variables|/Game/FGJ/AI/BP_Individual.BP_Individual_C|GetStatus _output_get)
        (:NewEnumerator0
          (Variables|Default|SetWaitingForPartner true))
        (:NewEnumerator1
          (CallFunction|SetupTable))))))

(fn SetupTable
  (Development|PrintString "TableSetu^p")
  (CallFunction|FindNewEmoji)
  (Variables|Default|SetCanGiveCake true)
  (Variables|Default|SetTableActive true)
  (switch Utilities|FlowControl|Switch|SwitchonEIndividualStatus (Variables|/Game/FGJ/AI/BP_Individual.BP_Individual_C|GetStatus (Variables|Default|GetIndividual1))
    (:NewEnumerator0
      (CallFunction|BeginRelationship))
    (:NewEnumerator1
      (CallFunction|BeginHeartbreak))))

(fn IndividualLeavingTable
  (params (Individual :type BP%20Individual%20Object%20Reference))
  (if (== Individual (Variables|Default|GetIndividual1))
    (Variables|Default|SetIndividual1 0)
    (CallFunction|EmptyTable)
    (else
      (Variables|Default|SetIndividual2 0))))

(fn EmptyTable
  (Variables|Default|SetTableActive false)
  (Variables|Default|SetTableTaken false)
  (Variables|Default|SetWaitingForPartner false)
  (Variables|Default|SetbIsChairOneTaken false)
  (Variables|BP_Table_C|SetCoupleIsBeside (Variables|Default|GetPairedTable) false))

(fn FindNewEmoji
  (bind _gamemode (Variables|Default|GetGameMode))
  (bind _emojilist (Variables|/Game/FGJ/Core/BP_MainGameMode.BP_MainGameMode_C|GetEmojiList _gamemode))
  (Variables|Default|SetCurrentEmoji (Utilities|Array|Get(acopy) (.array _emojilist) (Math|Random|RandomInteger (Utilities|Array|Length (.array _emojilist))))))

(fn GiveCake
  (params (Cake :type BP%20Cake%20Object%20Reference))
  (if (Variables|Default|GetCanGiveCake)
    (Variables|Default|SetCurrentCake Cake)
    (Variables|Default|SetCanGiveCake false)
    (Variables|Default|SetCurrentlyEatingCake true)
    (CallFunction|EatCake)))

(fn CakeEaten
  (Variables|Default|SetCanGiveCake true)
  (Variables|Default|SetCurrentlyEatingCake false)
  ;[1 1 1] Remove Cake - Add animation here
  (Actor|DestroyActor (Variables|Default|GetCurrentCake))
  (Variables|Default|SetCurrentCake 0))

(fn BeginRelationship
  (bind _relationshipaffinitystartrangepercent (Variables|Default|GetRelationshipAffinityStartRangePercent))
  (Variables|Default|SetRelationshipAffinity (Math|Float|Truncate (* (Variables|Default|GetMaxRelationshipAffinity) (Math|Random|RandomFloatinRange (.x _relationshipaffinitystartrangepercent) (.y _relationshipaffinitystartrangepercent)))))
  (Variables|Default|SetcanProgress true)
  (Development|PrintString "Beginning Relationship")
  (CallFunction|Progress))

(fn BeginHeartbreak
  (Development|PrintString "HEARTBREAK")
  (Variables|/Game/FGJ/AI/BP_Individual.BP_Individual_C|SetHeartbreakAffinity (Variables|Default|GetIndividual1) 0)
  (Variables|Default|SetcanProgress true)
  (CallFunction|Progress)
  (Variables|BP_Table_C|SetCoupleIsBeside (Variables|Default|GetPairedTable) false))

(fn ProgressRelationship
  (bind _relationshipchanceatpositiveprogress (Variables|Default|GetRelationshipChanceAtPositiveProgress))
  (bind _relationshipaffinity (Variables|Default|GetRelationshipAffinity))
  (Development|PrintString "Prog Relationship")
  (if (<= (Math|Random|RandomFloat) (Math|Random|RandomFloatinRange (.x _relationshipchanceatpositiveprogress) (.y _relationshipchanceatpositiveprogress)))
    (Math|Integer|IncrementInt _relationshipaffinity)
    (else
      (Math|Integer|DecrementInt _relationshipaffinity))))

(fn ProgressHeartbreak
  (Math|Integer|IncrementInt (Variables|/Game/FGJ/AI/BP_Individual.BP_Individual_C|GetHeartbreakAffinity (Variables|Default|GetIndividual1))
    (:%20%20
      (Development|PrintString "Heartbreak Progress"))))

(fn FinishRelationship
  (params (PositiveEnding :type Boolean))
  (bind _individual1 (Variables|Default|GetIndividual1))
  (Variables|Default|SetcanProgress false)
  (if PositiveEnding
    ;[1 1 1] Leave the Cafe - Stagger ?
    (Default|LeaveCafe (Variables|Default|GetIndividual1))
    (Default|LeaveCafe (Variables|Default|GetIndividual2))
    (CallFunction|EmptyTable)
    (else
      (Utilities|FlowControl|Sequence
        (:then_0
          (Utilities|Array|Add (Variables|/Game/FGJ/AI/BP_Individual.BP_Individual_C|GetIDOfHeartbreak _individual1) (Variables|/Game/FGJ/AI/BP_Individual.BP_Individual_C|GetIndividualID (Variables|Default|GetIndividual2))))
        (:then_1
          (Utilities|Array|Add (Variables|/Game/FGJ/AI/BP_Individual.BP_Individual_C|GetIDOfHeartbreak (Variables|Default|GetIndividual2)) (Variables|/Game/FGJ/AI/BP_Individual.BP_Individual_C|GetIndividualID _individual1)))
        (:then_2
          (Variables|/Game/FGJ/AI/BP_Individual.BP_Individual_C|SetStatus (Variables|Default|GetIndividual2) "NewEnumerator1")
          (bind _table (Default|FindAvailableTable (Variables|Default|GetGameMode) "NewEnumerator1"))
          (Default|MovetoTable (Variables|Default|GetIndividual2) _table)
          (Variables|Default|SetIndividual2 0))
        (:then_3
          (Variables|/Game/FGJ/AI/BP_Individual.BP_Individual_C|SetStatus (Variables|Default|GetIndividual1) "NewEnumerator1")
          (CallFunction|SetupTable))))))

(fn FinishHeartbreak
  (Variables|Default|SetcanProgress false)
  (Variables|Default|SetTableActive false)
  (Variables|/Game/FGJ/AI/BP_Individual.BP_Individual_C|SetStatus (Variables|Default|GetIndividual1) "NewEnumerator2")
  (Development|PrintString "Heartbreak Finished" true true "(R=0.000000,G=0.660000,B=1.000000,A=1.000000)" 2e+01))

(fn AddAffinity
  (params (Amount :type Integer))
  (bind _individual1 (Variables|Default|GetIndividual1))
  (switch Utilities|FlowControl|Switch|SwitchonEIndividualStatus (Variables|/Game/FGJ/AI/BP_Individual.BP_Individual_C|GetStatus _individual1)
    (:NewEnumerator0
      (Variables|Default|SetRelationshipAffinity (+ (Variables|Default|GetRelationshipAffinity) Amount)))
    (:NewEnumerator1
      (Variables|/Game/FGJ/AI/BP_Individual.BP_Individual_C|SetHeartbreakAffinity _individual1 (+ (Variables|/Game/FGJ/AI/BP_Individual.BP_Individual_C|GetHeartbreakAffinity _individual1) Amount)))))

(fn TableWaitingFinish
  (Variables|Default|SetTableActive false)
  (Variables|Default|SetCanGiveCake false)
  (Development|PrintString "Table Waiting To Finish"))