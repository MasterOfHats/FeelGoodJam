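; BP_MainGameMode is the game mode that tracks tables and scores how well an emoji matches a cake.
; BeginPlay caches every BP_Table actor in Tables.
; CalculateTags intersects cake tags with the emoji's primary and secondary tags, summing weighted matches and applying negative affinity for a tier with none.
; FindAvailableTable is unfinished: it checks for untaken tables but always returns false, leaving AssignTable unreachable.
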(event EventBeginPlay
  (bind _outactors (Actor|GetAllActorsOfClass "/Game/FGJ/Core/BP_Table.BP_Table_C"))
  (Variables|Default|SetTables _outactors))

(event EventTick
  (params (DeltaSeconds :type Float%20%28single-precision%29)))

(fn ConstructionScript)

(fn FindAvailableTable
  (params (Individual1 :type BP%20Table%20Object%20Reference) (Individual2 :type BP%20Table%20Object%20Reference))
  (for _array_element (Variables|Default|GetTables)
    (if (not (Variables|/Game/FGJ/Core/BP_Table.BP_Table_C|GetTableTaken _array_element))
      (if true
        _)))
  (return false 0))

(fn CalculateTags
  (params (Emoji :type Emoji%20Struct%20Structure) (Cake :type Cake%20Struct%20Structure))
  (bind _tags (Utilities|Struct|BreakCake_Struct Cake))
  (bind (_image _primarytags _secondarytags) (Utilities|Struct|BreakEmoji_Struct Emoji))
  (bind _secondarytagaffinityamount (Variables|Default|GetSecondaryTagAffinityAmount))
  (bind _primarytagaffinityamount (Variables|Default|GetPrimaryTagAffinityAmount))
  (bind _result (Utilities|Set|Intersection _primarytags _tags))
  (bind _result_2 (Utilities|Set|Intersection _secondarytags _tags))
  (return (+ (Math|Integer|SelectInt (* (Utilities|Set|Length _result) _primarytagaffinityamount) (* _primarytagaffinityamount -1) (!= (Utilities|Set|Length _result) 0)) (Math|Integer|SelectInt (* (Utilities|Set|Length _result_2) _secondarytagaffinityamount) (* _secondarytagaffinityamount -1) (!= (Utilities|Set|Length _result_2) 0)))))