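; BP_OvenFlicker is an actor that makes a referenced light flicker, presumably as oven glow going by its name.
; Each tick it interpolates the light component's intensity toward a target at a configurable speed.
; When the intensity nearly reaches that target, it picks a new random target within a fixed range, producing continuous, smooth, irregular flicker.
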(event EventBeginPlay)

(event Collision|EventActorBeginOverlap
  (params (OtherActor :type Actor%20Object%20Reference)))

(event EventTick
  (params (DeltaSeconds :type Float%20%28single-precision%29))
  (bind _light (Variables|Default|GetLight))
  (bind _lightcomponent (Variables|/Script/Engine.Light|GetLightComponent _light))
  (bind _intensity (Variables|/Script/Engine.LightComponentBase|GetIntensity _lightcomponent))
  (Rendering|Components|Light|SetIntensity _lightcomponent (Math|Interpolation|FInterpTo _intensity (Variables|Default|GetFlickerDestination) DeltaSeconds (Variables|Default|GetSpeed)))
  (if (Math|Float|NearlyEqual(Float) (Variables|Default|GetFlickerDestination) _intensity 0.001)
    (Variables|Default|SetFlickerDestination (Math|Random|RandomFloatinRange 0.5 1.0))))

(fn ConstructionScript)