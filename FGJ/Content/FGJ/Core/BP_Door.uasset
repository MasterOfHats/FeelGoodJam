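; Door actor that swings open with a doorbell and chime effect when a BP_Individual overlaps its EnterBox.
; A timeline rotates the door, with a Moving flag blocking retriggers mid-swing.
; Fully opening activates Leaf, plays a wind gust and starts a short timer, apparently for the reversing close.
; Fully closing plays a sound and resets the DoOnce that limits the bell to one ring per cycle.
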(event OnComponentBeginOverlap(EnterBox)
  (params (OverlappedComponent :type Primitive%20Component%20Object%20Reference) (OtherActor :type Actor%20Object%20Reference) (OtherComp :type Primitive%20Component%20Object%20Reference) (OtherBodyIndex :type Integer) (bFromSweep :type Boolean) (SweepResult :type Hit%20Result%20Structure%20%28by%20ref%29))
  (if (== (Utilities|GetClass OtherActor) "/Game/FGJ/AI/BP_Individual.BP_Individual_C")
    (CallFunction|OpenDoorEnter)
    (Utilities|FlowControl|DoOnce false
      (:Completed
        (Audio|PlaySoundatLocation "/Game/FGJ/Sounds/doorbell.doorbell" (Transformation|GetActorLocation) "0, 0, 0" 1.0 1.0 0.0 0 0 0)
        (Components|Activation|Activate (Variables|Default|GetChime) true)))))

(event Custom|ResetBell
  (Utilities|FlowControl|DoOnce false) ; enters at Reset
)

(event Custom|OpenDoorEnter
  (if (not (Variables|Default|GetbMoving))
    (Variables|Default|SetbMoving true)
    (bind (_direction _newtrack_0) (Timeline|Door Play)
      (:Update
        (Transformation|SetRelativeRotation (Variables|Default|GetDoorsies) (Math|Rotator|Lerp(Rotator) "0, 0, 0" "0,-110.000000, 0" _newtrack_0 true) false false))
      (:Finished
        (Variables|Default|SetbMoving false)
        (switch Utilities|FlowControl|Switch|SwitchonETimelineDirection _direction
          (:Forward
            (Utilities|Time|SetTimerbyEvent (EventDispatchers|CreateEvent :!event Custom|CloseDoorEnter) 2.0)
            (Components|Activation|Activate (Variables|Default|GetLeaf) true)
            (Audio|PlaySound2D "/Game/FGJ/Sounds/wind_gust__1_.wind_gust__1_" 1.0 1.0 0.0 0 0))
          (:Backward
            (CallFunction|ResetBell)
            (Audio|PlaySound2D "/Game/FGJ/Sounds/door_close.door_close" 1.0 1.0 0.0 0 0)))))))

(event Custom|CloseDoorEnter
  (if (not (Variables|Default|GetbMoving))
    (Variables|Default|SetbMoving true)
    (bind (_direction _newtrack_0) (Timeline|Door Reverse)
      (:Update
        (Transformation|SetRelativeRotation (Variables|Default|GetDoorsies) (Math|Rotator|Lerp(Rotator) "0, 0, 0" "0,-110.000000, 0" _newtrack_0 true) false false))
      (:Finished
        (Variables|Default|SetbMoving false)
        (switch Utilities|FlowControl|Switch|SwitchonETimelineDirection _direction
          (:Forward
            (Utilities|Time|SetTimerbyEvent (EventDispatchers|CreateEvent :!event Custom|CloseDoorEnter) 2.0)
            (Components|Activation|Activate (Variables|Default|GetLeaf) true)
            (Audio|PlaySound2D "/Game/FGJ/Sounds/wind_gust__1_.wind_gust__1_" 1.0 1.0 0.0 0 0))
          (:Backward
            (CallFunction|ResetBell)
            (Audio|PlaySound2D "/Game/FGJ/Sounds/door_close.door_close" 1.0 1.0 0.0 0 0)))))))

(fn ConstructionScript)