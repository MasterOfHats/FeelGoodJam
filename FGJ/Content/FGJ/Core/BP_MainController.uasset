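; Player controller for the witch cake-serving game, handling camera switches, cake pickup and delivery, and the seated ending.
; Interact blends between the default camera and table-zone cameras, with a timed lock and easing movement vectors to each view.
; In cake mode, cursor traces show cake descriptions and clicks put cakes on the witch's tray.
; Table cameras exit when she nears a screen edge; sitting after helping the couple triggers the ending.
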(event Custom|SetVectors
  (bind _returnvalue (Pawn|GetViewTarget))
  (bind _returnvalue_2 (Transformation|GetActorRightVector _returnvalue))
  (Variables|Default|SetPreviousForwardVector (Variables|Default|GetForwardVector))
  (Variables|Default|SetPreviousRightVector (Variables|Default|GetRightVector))
  (bind _newtrack_0 (Timeline|SettingVectors PlayFromStart)
    (:Update
      (Variables|Default|SetRightVector (Math|Vector|Lerp(Vector) (Variables|Default|GetPreviousRightVector) _returnvalue_2 _newtrack_0))
      (Variables|Default|SetForwardVector (Math|Vector|Lerp(Vector) (Variables|Default|GetPreviousForwardVector) (Math|Vector|CrossProduct _returnvalue_2 "0, 0,1.000000") _newtrack_0)))))

(event Custom|KeepCakeAtCursor
  (bind (_sizex _sizey) (HUD|GetViewportSize))
  (bind _cakemenu (Variables|Default|GetCakeMenu))
  (bind _root (Variables|/Game/FGJ/UI/WBP_CakeDescription.WBP_CakeDescription_C|GetRoot _cakemenu))
  (bind _returnvalue (Class|WidgetLayoutLibrary|SlotasCanvasSlot _root))
  (if (Utilities|IsValid (Variables|Default|GetCakeMenu))
    (bind _returnvalue_2 (Class|WidgetLayoutLibrary|GetMousePositiononViewport))
    (Utilities|FlowControl|Sequence
      (:then_0
        (if (Utilities|Enum|Equal(Enum) (Widget|GetVisibility (Variables|Default|GetCakeMenu)) "Hidden")
          (Class|CanvasPanelSlot|SetAlignment _returnvalue (Math|Vector2D|MakeVector2D (select (> (.X (Math|Vector2D|BreakVector2D (* _returnvalue_2 (Class|WidgetLayoutLibrary|GetViewportScale)))) (Math|Conversions|ToFloat(Integer) (/ _sizex 2))) 1.0 0.0) (select (> (.Y (Math|Vector2D|BreakVector2D (* _returnvalue_2 (Class|WidgetLayoutLibrary|GetViewportScale)))) (Math|Conversions|ToFloat(Integer) (/ _sizey 2))) 1.0 0.0)))))
      (:then_1
        (Class|CanvasPanelSlot|SetPosition _returnvalue _returnvalue_2)))))

(event Custom|CakeCheck
  (bind (_worldlocation _worlddirection) (Game|Player|ConvertMouseLocationToWorldSpace))
  (bind (_outhit _returnvalue) (Collision|LineTraceByChannel _worldlocation (+ _worldlocation (* _worlddirection 4e+02)) "TraceTypeQuery1" false (Utilities|Array|MakeArray (Variables|Default|GetWitchCharacter)) "None"))
  (if _returnvalue
    (if (not (Utilities|IsValid (Variables|Default|GetHeldCake)))
      (bind _asbp_cake (Utilities|Casting|CastToBP_Cake (.HitActor (Collision|BreakHitResult _outhit)))
        (:then
          (Widget|SetVisibility (Variables|Default|GetCakeMenu) "Visible")
          (Default|UpdateCake (Variables|Default|GetCakeMenu) _asbp_cake))
        (:CastFailed
          (Widget|SetVisibility (Variables|Default|GetCakeMenu) "Hidden" :!label _label)))
      (else
        (goto _label)))
    (else
      (goto _label))))

(event Custom|EndingEventHeart
  (Utilities|FlowControl|Delay 0.75)
  (Default|EndingEventFadeinHeart (Variables|Default|GetCurrentTable)))

(event Custom|EndingEvent
  (bind _witchcharacter (Variables|Default|GetWitchCharacter))
  (bind _currenttablezone (Variables|Default|GetCurrentTableZone))
  (bind _associatedtable (Variables|/Game/FGJ/Core/BP_TableZone.BP_TableZone_C|GetAssociatedTable _currenttablezone))
  (bind _chair1 (Variables|/Game/FGJ/Core/BP_Table.BP_Table_C|GetChair1 _associatedtable))
  (bind _returnvalue (Transformation|GetWorldTransform _chair1))
  (Variables|Default|SetPlayerHasControl false)
  (CallFunction|GotoTable _currenttablezone)
  (Variables|/Game/FGJ/Core/BP_Table.BP_Table_C|SetTableTaken _associatedtable true)
  (Default|Moveto _witchcharacter (Math|Transform|MakeTransform (Math|Vector|MakeVector (.x (.location _returnvalue)) (.y (.location _returnvalue)) (.z (Transformation|GetActorLocation _witchcharacter))) "0, 0, 0" "1,1,1")) ; Sets the character to the right position
  (bind _returnvalue_2 (Game|SpawnActorfromClass "/Game/FGJ/AI/BP_Individual.BP_Individual_C" (Math|Transform|MakeTransform "0, 0,-500.000000" "0, 0, 0" "1,1,1") "Undefined" 0 0))
  (Variables|/Game/FGJ/AI/BP_Individual.BP_Individual_C|SetStatus _returnvalue_2 "NewEnumerator1")
  (Variables|/Game/FGJ/Core/BP_Table.BP_Table_C|SetIndividual1 (Variables|/Game/FGJ/Core/BP_TableZone.BP_TableZone_C|GetAssociatedTable (Variables|Default|GetCurrentTableZone)) _returnvalue_2))

(event EventBeginPlay
  (bind _asbp_main_game_mode (Utilities|Casting|CastToBP_MainGameMode (Game|GetGameMode)))
  (Variables|Default|SetGameMode _asbp_main_game_mode)
  (Utilities|FlowControl|Sequence
    (:then_0
      (CallFunction|SelectFirstCam "NewEnumerator0" 0.0)
      (bind _asbp_witch_character (Utilities|Casting|CastToBP_WitchCharacter (Pawn|GetControlledPawn)))
      (Variables|Default|SetWitchCharacter _asbp_witch_character)
      (Variables|/Game/FGJ/Core/BP_WitchCharacter.BP_WitchCharacter_C|SetMainController _asbp_witch_character self)
      (CallFunction|SetVectors))
    (:then_1
      (bind _returnvalue (UserInterface|CreateWidget "/Game/FGJ/UI/WBP_CakeDescription.WBP_CakeDescription_C"))
      (UserInterface|Viewport|AddtoViewport _returnvalue 0)
      (bind _output_get (Variables|Default|SetCakeMenu _returnvalue))
      (Widget|SetVisibility _output_get "Hidden"))
    (:then_2
      (bind _returnvalue_2 (UserInterface|CreateWidget "/Game/FGJ/UI/WBP_Interact.WBP_Interact_C"))
      (UserInterface|Viewport|AddtoViewport _returnvalue_2 1)
      (bind _output_get_2 (Variables|Default|SetInteractUI _returnvalue_2))
      (Widget|SetVisibility _output_get_2 "Visible"))
    (:then_3
      (Class|PlayerController|SetAudioListenerAttenuationOverride (Variables|/Script/Engine.Character|GetCapsuleComponent (Variables|Default|GetWitchCharacter)) "0, 0, 0"))))

(event EventTick
  (params (DeltaSeconds :type Float%20%28single-precision%29))
  (bind _returnvalue (Game|Player|GetPlayerPawn 0))
  (bind (_sizex _sizey) (HUD|GetViewportSize))
  (bind _self self)
  (bind _returnvalue_2 (Math|Conversions|ToFloat(Integer) _sizey))
  (bind _returnvalue_3 (Transformation|GetActorLocation _returnvalue))
  (bind _returnvalue_4 (Math|Conversions|ToFloat(Integer) _sizex))
  (bind _screenposition (Class|GameplayStatics|ProjectWorldtoScreen _self _returnvalue_3 true))
  (bind _returnvalue_5 (/ (.y _screenposition) _returnvalue_2))
  (bind _returnvalue_6 (/ (.x _screenposition) _returnvalue_4))
  (if (Variables|Default|GetPlayerHasControl)
    (Utilities|FlowControl|Sequence
      (:then_0
        (CallFunction|KeepCakeatCursor)
        (if (and (Utilities|IsValid (Variables|Default|GetCurrentCam)) (not (Variables|Default|GetSwitching)))
          (if (Math|Boolean|ORBoolean (< _returnvalue_6 0.15) (> _returnvalue_6 0.85) (< _returnvalue_5 0.15) (> _returnvalue_5 0.85))
            (CallFunction|SelectFirstCam "NewEnumerator0" 1.0)
            (Variables|Default|SetCurrentCam 0)
            (Utilities|IsValid (Variables|Default|GetCurrentTable)
              (:Is%20Valid
                (Default|PlayerZoomedOutOfTable (Variables|Default|GetCurrentTable)))
              (:Is%20Not%20Valid
                _))
            (Variables|Default|SetCurrentTable 0))))
      (:then_1
        (if (Utilities|Enum|Equal(Enum) (Variables|Default|GetCurrentMode) "NewEnumerator1")
          (CallFunction|CakeCheck)
          (else
            (Widget|SetVisibility (Variables|Default|GetCakeMenu) "Hidden")))))))

(event Input|ActionEvents|InputActionInteract
  (params (Key :type Key%20Structure :default "None"))
  (bind _currenttablezone (Variables|Default|GetCurrentTableZone))
  ;[1 1 1] Switch to a table or back from cake-mode
  (:Pressed
    (if (Variables|Default|GetPlayerHasControl)
      (Utilities|IsValid _currenttablezone
        (:Is%20Valid
          (if (Math|Boolean|ANDBoolean (Utilities|IsValid (Variables|Default|GetHeldCake)) (Utilities|IsValid (Variables|Default|GetCurrentTable)) (Utilities|IsValid (Variables|Default|GetCurrentTableZone)))
            (if (== (Variables|/Game/FGJ/Core/BP_TableZone.BP_TableZone_C|GetAssociatedTable (Variables|Default|GetCurrentTableZone)) (Variables|Default|GetCurrentTable))
              (if (Variables|/Game/FGJ/Core/BP_Table.BP_Table_C|GetCanGiveCake (Variables|/Game/FGJ/Core/BP_TableZone.BP_TableZone_C|GetAssociatedTable (Variables|Default|GetCurrentTableZone)))
                (CallFunction|GiveCake (Variables|Default|GetHeldCake))
                (Default|FireSpawnCake (Variables|Default|GetGameMode)))
              (else
                (if (!= (Variables|/Game/FGJ/Core/BP_TableZone.BP_TableZone_C|GetAssociatedCamera _currenttablezone) (Pawn|GetViewTarget)) :!label _label
                  (if (not (Variables|Default|GetSwitching))
                    (CallFunction|GotoTable _currenttablezone)
                    (Utilities|IsValid (Variables|Default|GetCurrentTable)
                      (:Is%20Valid
                        (Default|PlayerZoomedinonTable (Variables|Default|GetCurrentTable)))))
                  (elif (not (Variables|Default|GetSwitching))
                    (Variables|Default|SetbShowMouseCursor false)
                    (CallFunction|SelectFirstCam "NewEnumerator0" 1.0)
                    (Variables|Default|SetCurrentCam 0)
                    (Utilities|IsValid (Variables|Default|GetCurrentTable)
                      (:Is%20Valid
                        (Default|PlayerZoomedOutOfTable (Variables|Default|GetCurrentTable)))
                      (:Is%20Not%20Valid
                        _))
                    (Variables|Default|SetCurrentTable 0)))))
            (else
              (goto _label))))))))

(event Input|ActionEvents|InputActionSitDown
  (params (Key :type Key%20Structure :default "None"))
  (bind _currenttablezone (Variables|Default|GetCurrentTableZone))
  (bind _associatedtable (Variables|/Game/FGJ/Core/BP_TableZone.BP_TableZone_C|GetAssociatedTable _currenttablezone))
  ;[1 1 1] On specific conditions play end sequence, this removes players control
  (:Pressed
    (if (Math|Boolean|ANDBoolean (Variables|/Game/FGJ/Core/BP_MainGameMode.BP_MainGameMode_C|GetHelpedCoupleGetTogether (Variables|Default|GetGameMode)) (Utilities|IsValid (Variables|Default|GetCurrentTableZone)) (not (Utilities|IsValid (Variables|Default|GetHeldCake))))
      (Utilities|IsValid _associatedtable
        (:Is%20Valid
          (if (not (Variables|/Game/FGJ/Core/BP_Table.BP_Table_C|GetTableTaken _associatedtable))
            (Default|StartEndSequence (Variables|Default|GetGameMode))))))))

(event Input|MouseEvents|LeftMouseButton
  (params (Key :type Key%20Structure :default "None"))
  (bind (_worldlocation _worlddirection) (Game|Player|ConvertMouseLocationToWorldSpace))
  (:Pressed
    (if (Variables|Default|GetPlayerHasControl)
      (if (Utilities|Enum|Equal(Enum) (Variables|Default|GetCurrentMode) "NewEnumerator1")
        (bind _outhit (Collision|LineTraceByChannel _worldlocation (+ _worldlocation (* _worlddirection 4e+02)) "TraceTypeQuery1" false (Utilities|Array|MakeArray (Variables|Default|GetWitchCharacter)) "None"))
        (if (not (Utilities|IsValid (Variables|Default|GetHeldCake)))
          (Development|PrintString (Utilities|GetDisplayName (.HitActor (Collision|BreakHitResult _outhit))) true true "(R=1.000000,G=0.000000,B=0.251891,A=1.000000)")
          (bind _asbp_cake (Utilities|Casting|CastToBP_Cake (.HitActor (Collision|BreakHitResult _outhit))))
          (CallFunction|TakeCake _asbp_cake))))))

(event Input|KeyboardEvents|SpaceBar
  (params (Key :type Key%20Structure :default "None"))
  ;[1 1 1] Switch to a table or back from cake-mode
)

(fn ConstructionScript)

(fn SelectFirstCam
  (params (CamType :type CameraMode%20Enum :default "NewEnumerator0") (BlendTime :type Float%20%28single-precision%29))
  (bind _outactors (Actor|GetAllActorsOfClass "/Game/FGJ/Core/BP_Camera.BP_Camera_C"))
  (for _array_element _outactors
    (if (Utilities|Enum|Equal(Enum) (Variables|/Game/FGJ/Core/BP_Camera.BP_Camera_C|GetCameraMode _array_element) CamType)
      (Variables|Default|SetCurrentMode (Variables|/Game/FGJ/Core/BP_Camera.BP_Camera_C|GetCameraMode _array_element))
      (Game|Player|SetViewTargetwithBlend _array_element BlendTime "VTBlend_Linear" 0.0 false)
      (CallFunction|SetVectors)
      (CallFunction|Switch)
      (return))))

(fn GotoTable
  (params (TableZone :type BP%20Table%20Zone%20Object%20Reference))
  (bind _returnvalue (Game|GetPlayerController 0))
  (bind _output_get (Variables|Default|SetCurrentTableZone TableZone))
  (if (Utilities|Enum|Equal(Enum) (Variables|/Game/FGJ/Core/BP_Camera.BP_Camera_C|GetCameraMode (Variables|/Game/FGJ/Core/BP_TableZone.BP_TableZone_C|GetAssociatedCamera _output_get)) "NewEnumerator2")
    (Variables|Default|SetCurrentCam (Variables|/Game/FGJ/Core/BP_TableZone.BP_TableZone_C|GetAssociatedCamera _output_get))
    (else
      ;[1 1 1] Ensures the cake camera has the right orientation
      (Transformation|SetActorRotation (Variables|/Game/FGJ/Core/BP_TableZone.BP_TableZone_C|GetAssociatedCamera _output_get))
      (Variables|Default|SetbShowMouseCursor true) ; Enables the cursor
    ))
  (Variables|Default|SetCurrentMode (Variables|/Game/FGJ/Core/BP_Camera.BP_Camera_C|GetCameraMode (Variables|/Game/FGJ/Core/BP_TableZone.BP_TableZone_C|GetAssociatedCamera _output_get)))
  (Game|Player|SetViewTargetwithBlend _returnvalue (Variables|/Game/FGJ/Core/BP_TableZone.BP_TableZone_C|GetAssociatedCamera _output_get) (Variables|/Game/FGJ/Core/BP_TableZone.BP_TableZone_C|GetBlendTime (Variables|Default|GetCurrentTableZone)) "VTBlend_Linear" 0.0 false)
  (bind _asbp_witch_character (Utilities|Casting|CastToBP_WitchCharacter (Pawn|GetControlledPawn _returnvalue)))
  ;[1 1 1] Final setups for the camera switch
  (Variables|Default|SetCurrentTable (Variables|/Game/FGJ/Core/BP_TableZone.BP_TableZone_C|GetAssociatedTable (Variables|Default|GetCurrentTableZone)))
  (Default|Moveto _asbp_witch_character (Transformation|GetWorldTransform (Variables|/Game/FGJ/Core/BP_TableZone.BP_TableZone_C|GetLocation (Variables|Default|GetCurrentTableZone)))) ; Sets the character to the right position
  (CallFunction|SetVectors) ; Ajusts the movement orientation
  (CallFunction|Switch) ; Times a boolean so you can't switch back\nduring the blend
)

(fn Switch
  (if (Variables|Default|GetSwitching)
    (Variables|Default|SetSwitching false)
    (else
      (Variables|Default|SetSwitching true)
      (Utilities|Time|SetTimerbyFunctionName self "Switch" 1.0))))

(fn TakeCake
  (params (Cake :type BP%20Cake%20Object%20Reference))
  (Transformation|AttachComponentToComponent Cake (Variables|/Game/FGJ/Core/BP_WitchCharacter.BP_WitchCharacter_C|GetCakeLocation (Variables|Default|GetWitchCharacter)) "None" "SnapToTarget" "SnapToTarget" "KeepWorld" true)
  (Variables|Default|SetHeldCake Cake)
  (Development|SetHiddeninGame (Variables|/Game/FGJ/Core/BP_WitchCharacter.BP_WitchCharacter_C|GetTray (Variables|Default|GetWitchCharacter)) false true)
  (Components|StaticMesh|SetStaticMesh (Variables|/Game/FGJ/Core/Cakes/BP_Cake.BP_Cake_C|GetCakeMesh Cake) (.mesh (Variables|/Game/FGJ/Core/Cakes/BP_Cake.BP_Cake_C|GetCakeStruct (Variables|Default|GetHeldCake))))
  (bind _returnvalue (Actor|GetActorOfClass "/Game/FGJ/Sounds/BP_KentNagano.BP_KentNagano_C"))
  (Default|SoloSwitch _returnvalue false (.name (Variables|/Game/FGJ/Core/Cakes/BP_Cake.BP_Cake_C|GetCakeStruct (Variables|Default|GetHeldCake))))
  (Audio|PlaySound2D "/Game/FGJ/Sounds/cake_disappearing.cake_disappearing" 1.0 1.0 0.0 0 0))

(fn GiveCake
  (params (Cake :type BP%20Cake%20Object%20Reference))
  (Transformation|DetachFromActor (Variables|Default|GetHeldCake) "KeepRelative" "KeepRelative" "KeepRelative")
  (Default|GiveCake (Variables|/Game/FGJ/Core/BP_TableZone.BP_TableZone_C|GetAssociatedTable (Variables|Default|GetCurrentTableZone)) (Variables|Default|GetHeldCake))
  (Variables|Default|SetHeldCake 0)
  (Development|SetHiddeninGame (Variables|/Game/FGJ/Core/BP_WitchCharacter.BP_WitchCharacter_C|GetTray (Variables|Default|GetWitchCharacter)) true true))

(fn StartEndSequence
  (CallFunction|EndingEvent))