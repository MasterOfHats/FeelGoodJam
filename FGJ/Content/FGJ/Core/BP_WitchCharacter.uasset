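; Player witch character that handles movement input and facing, driven by the main controller's control state and direction vectors.
; Tick smooths yaw toward velocity with wrap-around correction instead of Unreal's built-in orientation, and copies the cake camera's yaw when idle in cake mode.
; MoveTo runs a timeline that lerps the actor's transform to a target, such as a table, blocking movement input meanwhile.
; GiveCake is an empty stub.
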(event Custom|MoveTo
  (params (TargetLocation :type Transform))
  ;[1 1 1] Simple forceful move to for tables
  (Variables|Default|SetTargetLocation TargetLocation)
  (Variables|Default|SetbMovingTo true)
  (Variables|Default|SetInitialLocation (Transformation|GetActorTransform))
  (bind _newtrack_0 (Timeline|MovingTo PlayFromStart)
    (:Update
      (Transformation|SetActorTransform (Math|Transform|Lerp(Transform) (Variables|Default|GetInitialLocation) (Variables|Default|GetTargetLocation) _newtrack_0)))
    (:Finished
      (Variables|Default|SetbMovingTo false))))

(event EventTick
  (params (DeltaSeconds :type Float%20%28single-precision%29))
  (bind _charactermovement (Variables|Character|GetCharacterMovement))
  (bind _maincontroller (Variables|Default|GetMainController))
  (bind _velocity (Variables|/Script/Engine.MovementComponent|GetVelocity _charactermovement))
  (bind _returnvalue (Math|Rotator|MakeRotfromXZ _velocity (Math|Vector|MakeVector 0.0 0.0 1.0)))
  (if (Variables|/Game/FGJ/Core/BP_MainController.BP_MainController_C|GetPlayerHasControl (Variables|Default|GetMainController))
    (if (> (Math|Vector|VectorLength (Variables|/Script/Engine.MovementComponent|GetVelocity (Variables|Character|GetCharacterMovement))) 5.0)
      ;[1 1 1] Orients player rotation to movement. Uses a smoother change than Unreal's base method
      (bind _output_get (Variables|Default|SetYaw (Math|Interpolation|FInterpTo (Math|Float|SelectFloat (Variables|Default|GetYaw) (+ (Variables|Default|GetYaw) (Math|Float|SelectFloat -3.6e+02 3.6e+02 (< (Math|Float|Absolute(Float) (- (.yaw _returnvalue) (- (Variables|Default|GetYaw) 3.6e+02))) (Math|Float|Absolute(Float) (- (.yaw _returnvalue) (+ (Variables|Default|GetYaw) 3.6e+02)))))) (< (Math|Float|Absolute(Float) (- (.yaw _returnvalue) (Variables|Default|GetYaw))) (Math|Float|Absolute(Float) (- (.yaw _returnvalue) (+ (Variables|Default|GetYaw) (Math|Float|SelectFloat -3.6e+02 3.6e+02 (< (Math|Float|Absolute(Float) (- (.yaw _returnvalue) (- (Variables|Default|GetYaw) 3.6e+02))) (Math|Float|Absolute(Float) (- (.yaw _returnvalue) (+ (Variables|Default|GetYaw) 3.6e+02)))))))))) (.yaw _returnvalue) DeltaSeconds 15.0)))
      (Transformation|SetActorRotation (Math|Rotator|MakeRotator 0.0 0.0 _output_get))
      (else
        ;[1 1 1] In cake mode the orientation is the same as the cake camera
        (if (Utilities|Enum|Equal(Enum) (Variables|/Game/FGJ/Core/BP_MainController.BP_MainController_C|GetCurrentMode _maincontroller) "NewEnumerator1")
          (bind _output_get_2 (Variables|Default|SetYaw (.yaw (Transformation|GetActorRotation (Pawn|GetViewTarget _maincontroller)))))
          (Transformation|SetActorRotation (Math|Rotator|MakeRotator 0.0 0.0 _output_get_2)))))))

(event Input|AxisEvents|InputAxisMoveUp
  (params (AxisValue :type Float%20%28single-precision%29))
  ;[1 1 1] Basic player movement
  (if (Variables|/Game/FGJ/Core/BP_MainController.BP_MainController_C|GetPlayerHasControl (Variables|Default|GetMainController))
    (if (not (Variables|Default|GetbMovingTo))
      (if (not (Variables|/Script/Engine.PlayerController|GetbShowMouseCursor (Variables|Default|GetMainController)))
        (Pawn|Input|AddMovementInput (Variables|/Game/FGJ/Core/BP_MainController.BP_MainController_C|GetForwardVector (Variables|Default|GetMainController)) AxisValue false)))))

(event Input|AxisEvents|InputAxisMoveRight
  (params (AxisValue :type Float%20%28single-precision%29))
  ;[1 1 1] Basic player movement
  (if (Variables|/Game/FGJ/Core/BP_MainController.BP_MainController_C|GetPlayerHasControl (Variables|Default|GetMainController))
    (if (not (Variables|Default|GetbMovingTo))
      (if (not (Variables|/Script/Engine.PlayerController|GetbShowMouseCursor (Variables|Default|GetMainController)))
        (Pawn|Input|AddMovementInput (Variables|/Game/FGJ/Core/BP_MainController.BP_MainController_C|GetRightVector (Variables|Default|GetMainController)) AxisValue false)))))

(fn ConstructionScript)

(fn QInterpto
  (params (QuaternionA :type Quat%20Structure) (QuaternionB :type Quat%20Structure) (DeltaTime :type Float%20%28single-precision%29) (InterpSpeed :type Float%20%28single-precision%29))
  (bind (_x _y _z _w) (Utilities|Struct|BreakQuat QuaternionB))
  (bind (_x_2 _y_2 _z_2 _w_2) (Utilities|Struct|BreakQuat QuaternionA))
  (return (Utilities|Struct|MakeQuat (Math|Interpolation|FInterpTo _x_2 _x DeltaTime InterpSpeed) (Math|Interpolation|FInterpTo _y_2 _y DeltaTime InterpSpeed) (Math|Interpolation|FInterpTo _z_2 _z DeltaTime InterpSpeed) (Math|Interpolation|FInterpTo _w_2 _w DeltaTime InterpSpeed))))

(fn GiveCake)