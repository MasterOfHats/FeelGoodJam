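; Cafe customer pawn with a random color and name, seated at tables and tracking a relationship status (looking, waiting, in relationship, heartbroken).
; BP_IndividualController handles movement to chairs and out of the cafe, while the pawn notifies tables when moving, leaving or sitting.
; Status drives timeline-based procedural animation: periodic hops when in a relationship, leaning toward the table when waiting or heartbroken.
; Tick accumulates waiting time, resetting it in other states.
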(event Custom|StartMove
  (Transformation|SetRelativeRotation (Variables|Default|GetBody) "-20.000000, 0, 0" false false)
  (bind _height (Timeline|Timeline_0 PlayFromStart)
    (:Update
      (Transformation|SetRelativeLocation (Variables|Default|GetBody) (Math|Vector|MakeVector 0.0 0.0 (Math|Float|Lerp 0.0 -25.0 _height)) false false))))

(event Custom|StopMove
  (Transformation|SetRelativeRotation (Variables|Default|GetBody) "0, 0, 0" false false)
  (Transformation|SetRelativeLocation (Variables|Default|GetBody) "0, 0, 0" false false)
  (bind _height (Timeline|Timeline_0 Stop)
    (:Update
      (Transformation|SetRelativeLocation (Variables|Default|GetBody) (Math|Vector|MakeVector 0.0 0.0 (Math|Float|Lerp 0.0 -25.0 _height)) false false))))

(event Custom|LeanOff
  (bind _body (Variables|Default|GetBody))
  (bind _height (Timeline|Timeline_2 Reverse)
    (:Update
      (Transformation|SetRelativeRotation _body (Math|Rotator|MakeRotator 0.0 (Math|Float|Lerp 0.0 -3e+01 _height) (.yaw (Math|Rotator|FindLookatRotation (Transformation|GetWorldLocation _body) (Transformation|GetActorLocation (Variables|Default|GetCurrentTable))))) false false)
      (Transformation|SetRelativeLocation (Variables|Default|GetLHand) (Math|Vector|Lerp(Vector) (Variables|Default|GetLHandStart) "117.000000,-43.000000,88.000000" _height) false false)
      (Transformation|SetRelativeLocation (Variables|Default|GetRHand) (Math|Vector|Lerp(Vector) (Variables|Default|GetRHandStart) "117.000000,76.000000,88.000000" _height) false false))))

(event Custom|LeanOn
  (bind _body (Variables|Default|GetBody))
  (bind _height (Timeline|Timeline_2 PlayFromStart)
    (:Update
      (Transformation|SetRelativeRotation _body (Math|Rotator|MakeRotator 0.0 (Math|Float|Lerp 0.0 -3e+01 _height) (.yaw (Math|Rotator|FindLookatRotation (Transformation|GetWorldLocation _body) (Transformation|GetActorLocation (Variables|Default|GetCurrentTable))))) false false)
      (Transformation|SetRelativeLocation (Variables|Default|GetLHand) (Math|Vector|Lerp(Vector) (Variables|Default|GetLHandStart) "117.000000,-43.000000,88.000000" _height) false false)
      (Transformation|SetRelativeLocation (Variables|Default|GetRHand) (Math|Vector|Lerp(Vector) (Variables|Default|GetRHandStart) "117.000000,76.000000,88.000000" _height) false false))))

(event Custom|Jumpies
  (bind _height (Timeline|Timeline_1 PlayFromStart)
    (:Update
      (Transformation|SetRelativeLocation (Variables|Default|GetBody) (Math|Vector|MakeVector 0.0 0.0 (Math|Float|Lerp 0.0 25.0 _height)) false false))))

(event EventBeginPlay
  (bind _asbp_individual_controller (Utilities|Casting|CastToBP_IndividualController (Pawn|GetController)))
  (bind _output_get (Variables|Default|SetAIController _asbp_individual_controller))
  (Variables|/Game/FGJ/AI/BP_IndividualController.BP_IndividualController_C|SetControlledPawn _output_get self)
  (bind _returnvalue (Rendering|Material|CreateDynamicMaterialInstance (Variables|Default|GetHead) 0 "/Game/FGJ/AI/M_Individuals_PH.M_Individuals_PH" "None" :!class /Script/Engine.PrimitiveComponent))
  (bind _output_get_2 (Variables|Default|SetMaterial _returnvalue))
  (Rendering|Material|SetMaterial (Variables|Default|GetBody) 0 _output_get_2)
  (Rendering|Material|SetVectorParameterValue (Variables|Default|GetMaterial) "Color" (Utilities|Select :Index (Math|Random|RandomIntegerinRange 0 9) :Option%200 "(R=1.000000,G=1.000000,B=1.000000,A=1.000000)" :Option%201 "(R=0.696878,G=0.683189,B=1.000000,A=1.000000)" :Option%202 "(R=0.973681,G=0.617977,B=1.000000,A=1.000000)" :Option%203 "(R=1.000000,G=0.555000,B=0.675994,A=1.000000)" :Option%204 "(R=1.000000,G=0.913360,B=0.399707,A=1.000000)" :Option%205 "(R=0.702019,G=1.000000,B=0.364242,A=1.000000)" :Option%206 "(R=0.410284,G=1.000000,B=0.465868,A=1.000000)" :Option%207 "(R=0.514087,G=1.000000,B=0.749239,A=1.000000)" :Option%208 "(R=0.228534,G=0.970150,B=1.000000,A=1.000000)" :Option%209 "(R=0.329358,G=0.475913,B=1.000000,A=1.000000)") :!class /Script/Engine.MaterialInstanceDynamic)
  (CallFunction|GenerateName)
  (bind _aswbp_name_ui (Utilities|Casting|CastToWBP_NameUI (UserInterface|GetUserWidgetObject (Variables|Default|GetWidget))))
  (bind _output_get_3 (Variables|Default|SetNameUI _aswbp_name_ui))
  (Rendering|Components|TextRender|SetText (Variables|/Game/FGJ/AI/WBP_NameUI.WBP_NameUI_C|GetName _output_get_3) (Utilities|Text|ToText(Name) (Variables|Default|GetName)))
  (Widget|SetRenderOpacity (Variables|Default|GetNameUI) 0.0)
  (Variables|Default|SetLHandStart (Variables|/Script/Engine.SceneComponent|GetRelativeLocation (Variables|Default|GetLHand)))
  (Variables|Default|SetRHandStart (Variables|/Script/Engine.SceneComponent|GetRelativeLocation (Variables|Default|GetRHand))))

(event EventTick
  (params (DeltaSeconds :type Float%20%28single-precision%29))
  (switch Utilities|FlowControl|Switch|SwitchonEIndividualStatus (Variables|Default|GetStatus)
    (:NewEnumerator0
      (Variables|Default|SetTimeWaiting 0.0 :!label _label))
    (:NewEnumerator1
      (goto _label))
    (:NewEnumerator2
      (Variables|Default|SetTimeWaiting (+ (Variables|Default|GetTimeWaiting) (Utilities|Time|GetWorldDeltaSeconds))))
    (:NewEnumerator3
      (goto _label))))

(fn ConstructionScript)

(fn GenerateName
  (Variables|Default|SetName (Utilities|Select :Index (Math|Random|RandomIntegerinRange 0 29) :Option%200 "Abrielle" :Option%201 "Bastian" :Option%202 "Destin" :Option%203 "Cassiel" :Option%204 "Evelynn" :Option%205 "Griffin" :Option%206 "Hannelore" :Option%207 "Ignacia" :Option%208 "Jessalyn" :Option%209 "Kyra" :Option%2010 "Liora" :Option%2011 "Lucius" :Option%2012 "Mireille" :Option%2013 "Nyssa" :Option%2014 "Odette" :Option%2015 "Peregrine" :Option%2016 "Qadira" :Option%2017 "Riona" :Option%2018 "Seraphim" :Option%2019 "Sorcha" :Option%2020 "Thalia" :Option%2021 "Uriel" :Option%2022 "Vespos" :Option%2023 "Yadira" :Option%2024 "Zaira" :Option%2025 "Eliron" :Option%2026 "Maylea" :Option%2027 "Oleisa" :Option%2028 "Xylia" :Option%2029 "Zaniel"))
  (return "Temp Name"))

(fn MovetoTable
  (params (Table :type BP%20Table%20Object%20Reference) (DelayBeforeMoving :type Float%20%28single-precision%29))
  (Utilities|Time|ClearTimerbyFunctionName 0 "JumpiesTimer")
  (Utilities|IsValid (Variables|Default|GetCurrentTable)
    (:Is%20Valid
      (Default|IndividualLeavingTable (Variables|Default|GetCurrentTable) self))
    (:Is%20Not%20Valid
      _))
  (bind _output_get (Variables|Default|SetCurrentTable Table))
  ;[1 1 1] Send Individuals to move to the table
  (Default|IndividualMovingtoTable _output_get self)
  (Default|MovetoChair (Variables|Default|GetAIController) (select (Variables|/Game/FGJ/Core/BP_Table.BP_Table_C|GetIsChairOneTaken _output_get) (Variables|/Game/FGJ/Core/BP_Table.BP_Table_C|GetChair1Seat _output_get) (Variables|/Game/FGJ/Core/BP_Table.BP_Table_C|GetChair2Seat _output_get)) DelayBeforeMoving)
  (Variables|/Game/FGJ/Core/BP_Table.BP_Table_C|SetIsChairOneTaken _output_get true)
  (CallFunction|StartMove))

(fn LeaveCafe
  (Default|LeaveCafe (Variables|Default|GetAIController))
  (Utilities|Time|ClearTimerbyFunctionName 0 "JumpiesTimer"))

(fn ReachedTable
  (Default|IndividualSatDown (Variables|Default|GetCurrentTable) self)
  (CallFunction|StopMove)
  (Transformation|SetActorRotation "0, 0, 0"))

(fn JumpiesTimer
  (CallFunction|Jumpies)
  (Utilities|Time|SetTimerbyFunctionName 0 "JumpiesTimer" (Math|Random|RandomFloatinRange 3.0 5.0)))

(fn SetIndividualID
  (params (ID :type Integer))
  (bind _output_get (Variables|Default|SetIndividualID ID))
  (Utilities|Array|Add (Variables|Default|GetIDOfHeartbreak) _output_get))

(fn StartingAState
  (switch Utilities|FlowControl|Switch|SwitchonEIndividualStatus (Variables|Default|GetStatus)
    (:NewEnumerator0
      (Utilities|Time|SetTimerbyFunctionName 0 "JumpiesTimer" (Math|Random|RandomFloatinRange 3.0 5.0))
      (CallFunction|LeanOff))
    (:NewEnumerator1
      (Utilities|Time|ClearTimerbyFunctionName 0 "JumpiesTimer" :!label _label)
      (CallFunction|Leanon))
    (:NewEnumerator2
      (goto _label))))