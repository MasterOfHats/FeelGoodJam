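; BP_IndividualController is the AI controller for BP_Individual pawns, moving them to café chairs or out of the café.
; On BeginPlay it caches the pawn and the level's BP_SpawnPoint, then immediately starts LeaveCafe.
; MoveToChair uses AIMoveTo to reach a given chair and notifies the pawn with ReachedTable on success.
; LeaveCafe walks the pawn to the spawn point, then has BP_MainGameMode despawn it.
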(event Custom|MoveToChair
  (params (Chair :type Static%20Mesh%20Component%20Object%20Reference))
  (AI|AIMoveTo 0 (Transformation|GetWorldLocation Chair) 0 5.0 false
    (:OnSuccess
      (Default|ReachedTable (Variables|Default|GetControlledPawn)))))

(event Custom|LeaveCafe
  (AI|AIMoveTo 0 (Transformation|GetActorLocation (Variables|Default|GetSpawnPoint)) 0 5.0 false
    (:OnSuccess
      (bind _asbp_main_game_mode (Utilities|Casting|CastToBP_MainGameMode (Game|GetGameMode)))
      (Default|DespawnIndividual _asbp_main_game_mode (Variables|Default|GetControlledPawn)))))

(event EventBeginPlay
  (bind _asbp_individual (Utilities|Casting|CastToBP_Individual (Pawn|GetControlledPawn)))
  (Variables|Default|SetControlledPawn _asbp_individual)
  (bind _returnvalue (Actor|GetActorOfClass "/Game/FGJ/AI/BP_SpawnPoint.BP_SpawnPoint_C"))
  (Variables|Default|SetSpawnPoint _returnvalue)
  (CallFunction|LeaveCafe))

(fn ConstructionScript)