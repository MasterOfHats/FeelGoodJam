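; BP_KentNagano is a music conductor that crossfades a solo instrument track to match the current cake.
; SoloSwitch stores the cake and table state, then Tick fades SoloTrack out, swaps its sound and fades it back in.
; Leaving the table selects a piano melody by Intensity; otherwise the cake picks the instrument, though some cakes have none.
; BeginPlay runs a timed, hardcoded sequence of switches, apparently as a test.
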(event Custom|SoloSwitch
  (params (bLeavingTable :type Boolean) (Cake :type ECakes%20Enum :default "NewEnumerator0"))
  (Variables|Default|SetNewCakeSolo Cake)
  (Variables|Default|SetbLeavingTable bLeavingTable)
  (Variables|Default|SetSoloStatus "NewEnumerator2"))

(event EventBeginPlay
  (Utilities|FlowControl|Delay 5.0)
  (CallFunction|SoloSwitch false "NewEnumerator14")
  (Utilities|FlowControl|Delay 6.0)
  (CallFunction|SoloSwitch false "NewEnumerator4")
  (Utilities|FlowControl|Delay 8.0)
  (CallFunction|SoloSwitch true "NewEnumerator4"))

(event EventTick
  (params (DeltaSeconds :type Float%20%28single-precision%29))
  (switch Utilities|FlowControl|Switch|SwitchonESoloStatus (Variables|Default|GetSoloStatus)
    (:NewEnumerator1
      (CallFunction|ChangeSoloVolume true))
    (:NewEnumerator2
      (CallFunction|ChangeSoloVolume false))))

(fn ConstructionScript)

(fn ChangeSoloVolume
  (params (bFadeIn :type Boolean))
  (bind _returnvalue (Math|Float|SelectFloat 1.0 -1.0 bFadeIn))
  (bind _returnvalue_2 (Utilities|Time|GetWorldDeltaSeconds))
  (bind _solotrack (Variables|Default|GetSoloTrack))
  (bind _cakesolofadetime (Variables|Default|GetCakeSoloFadeTime))
  (bind _returnvalue_3 (/ 1.0 _cakesolofadetime))
  (bind _volumemultiplier (Variables|/Script/Engine.AudioComponent|GetVolumeMultiplier _solotrack))
  (bind _returnvalue_4 (* _returnvalue_3 _returnvalue _returnvalue_2))
  (bind _returnvalue_5 (+ _volumemultiplier _returnvalue_4))
  (bind _returnvalue_6 (Math|Float|Clamp(Float) _returnvalue_5))
  (Audio|Components|Audio|SetVolumeMultiplier (Variables|Default|GetSoloTrack) _returnvalue_6 :!class /Script/Engine.AudioComponent)
  (if (== _returnvalue_6 (select bFadeIn 1.0 0.0))
    (switch Utilities|FlowControl|Switch|SwitchonESoloStatus (Variables|Default|GetSoloStatus)
      (:NewEnumerator1
        (Variables|Default|SetSoloStatus "NewEnumerator0"))
      (:NewEnumerator2
        (Variables|Default|SetSoloStatus "NewEnumerator1")
        (CallFunction|ChangeSoloSound)))))

(fn ChangeSoloSound
  (Audio|Components|Audio|SetSound (Variables|Default|GetSoloTrack) (select (Variables|Default|GetbLeavingTable) (Utilities|Select :Index (Variables|Default|GetIntensity) :Option%200 "/Game/FGJ/Sounds/PianoMelodyLight_6-8_75bpm_8m.PianoMelodyLight_6-8_75bpm_8m" :Option%201 "/Game/FGJ/Sounds/PianoMelodyMedium_6-8_75bpm_8m.PianoMelodyMedium_6-8_75bpm_8m" :Option%202 "/Game/FGJ/Sounds/PianoMelodyFull_6-8_75bpm_8m.PianoMelodyFull_6-8_75bpm_8m") (Utilities|Select :Index (Variables|Default|GetNewCakeSolo) :NewEnumerator0 0 :NewEnumerator1 0 :NewEnumerator2 0 :NewEnumerator3 0 :NewEnumerator4 "/Game/FGJ/Sounds/Violin_6-8_75bpm_16m.Violin_6-8_75bpm_16m" :NewEnumerator5 "/Game/FGJ/Sounds/Shamisen_6-8_75bpm_16m.Shamisen_6-8_75bpm_16m" :NewEnumerator6 0 :NewEnumerator7 0 :NewEnumerator8 "/Game/FGJ/Sounds/PanFlute_6-8_75bpm_16m.PanFlute_6-8_75bpm_16m" :NewEnumerator9 "/Game/FGJ/Sounds/Vibraphone_6-8_75bpm_16m.Vibraphone_6-8_75bpm_16m" :NewEnumerator10 "/Game/FGJ/Sounds/Flute_6-8_75bpm_16m.Flute_6-8_75bpm_16m" :NewEnumerator11 0 :NewEnumerator12 0 :NewEnumerator13 "/Game/FGJ/Sounds/Kalimba_6-8_75bpm_16m.Kalimba_6-8_75bpm_16m" :NewEnumerator14 "/Game/FGJ/Sounds/Theremin_6-8_75bpm_16m.Theremin_6-8_75bpm_16m" :NewEnumerator15 "/Game/FGJ/Sounds/Clarinet_6-8_75bpm_16m.Clarinet_6-8_75bpm_16m"))))